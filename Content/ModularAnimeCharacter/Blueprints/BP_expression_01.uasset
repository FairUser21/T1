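; BP_expression_01 is a modular anime character Blueprint that shows a fixed facial expression of widened eyes, a smile and lifted brows.
; On BeginPlay it sets hard-coded morph targets once on the Face and Eyebrows mesh components, with no blending or runtime updates.
; Unconnected nodes for an open mouth and raised inner brows never run, and the construction script is empty.
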(event `self.ReceiveBeginPlay`
  (bind _face (`self.Face`))
  (bind _eyebrows (`self.Eyebrows`))
  (`SkeletalMeshComponent.SetMorphTarget` _face "right eye widen 01" 1.0 true)
  (`SkeletalMeshComponent.SetMorphTarget` _face "left eye widen 01" 1.0 true)
  (`SkeletalMeshComponent.SetMorphTarget` _face "mouth smile 01" 1.0 true)
  (`SkeletalMeshComponent.SetMorphTarget` _eyebrows "left middle lift" 1.0 true)
  (`SkeletalMeshComponent.SetMorphTarget` _eyebrows "right middle lift" 0.9 true))

(fn `UserConstructionScript`)
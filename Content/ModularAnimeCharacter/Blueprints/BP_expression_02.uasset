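; Modular anime character Blueprint that poses an angry, shouting facial expression.
; On BeginPlay it sets fixed morph target weights once on the Face and Eyebrows components, combining angry eyes, a shouting mouth shape and lowered brows, slightly asymmetric between left and right.
; The Mouth component call names no morph target, and the construction script, overlap and Tick events are empty.
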(event `self.ReceiveBeginPlay`
  (bind _face (`self.Face`))
  (bind _eyebrows (`self.Eyebrows`))
  (`SkeletalMeshComponent.SetMorphTarget` _face "left eye angry" 1.0 true)
  (`SkeletalMeshComponent.SetMorphTarget` _face "left eye lower lid up" 0.5 true)
  (`SkeletalMeshComponent.SetMorphTarget` _face "right eye angry" 1.0 true)
  (`SkeletalMeshComponent.SetMorphTarget` _face "mouth shout 04" 1.0 true)
  (`SkeletalMeshComponent.SetMorphTarget` (`self.Mouth`) "None" 0.0 true)
  (`SkeletalMeshComponent.SetMorphTarget` _eyebrows "left angry" 1.0 true)
  (`SkeletalMeshComponent.SetMorphTarget` _eyebrows "right angry" 1.0 true)
  (`SkeletalMeshComponent.SetMorphTarget` _eyebrows "left inner down" 1.0 true)
  (`SkeletalMeshComponent.SetMorphTarget` _eyebrows "left down" 0.8 true)
  (`SkeletalMeshComponent.SetMorphTarget` _eyebrows "right down" 1.0 true))

(fn `UserConstructionScript`)
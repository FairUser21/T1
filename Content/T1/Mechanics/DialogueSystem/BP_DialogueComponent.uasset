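; Actor component that runs data-table-driven dialogue, showing lines and selectable replies in a WB_Dialogue widget.
; Interact opens the widget with mouse cursor or advances it, each row supplying the next row, table and end flag.
; An open-ended opening row spawns WB_Options buttons, and Optionselected jumps to the chosen row.
; LeaveDialogue, or Interact after an end row, removes the widget and restores game-only input.
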(event `/Game/T1/Mechanics/DialogueSystem/BP_Interact.LeaveDialogue`
  (bind _returnvalue (`GameplayStatics.GetPlayerController` 0))
  (`/Engine/EditorBlueprintResources/StandardMacros.IsValid` (`self.WidgetDialogue`)
    (:`Is Valid`
      (`Widget.RemoveFromParent` (`self.WidgetDialogue`) :!label _label)
      (set `self.EndDialogue` false)
      (set `self.WidgetDialogue` null)
      (`WidgetBlueprintLibrary.SetInputMode_GameOnly` _returnvalue)
      (set `PlayerController.bShowMouseCursor` false _returnvalue))))

(event `/Game/T1/Mechanics/DialogueSystem/BP_Interact.Interact`
  (params (playerRef :type "/Game/ThirdPerson/Blueprints/BP_ThirdPersonCharacter Object Reference"))
  (bind _returnvalue (`GameplayStatics.GetPlayerController` 0))
  (if (`self.EndDialogue`)
    (goto _label)
    (else
      (`/Engine/EditorBlueprintResources/StandardMacros.IsValid` (`self.WidgetDialogue`)
        (:`Is Valid`
          (bind _returnvalue_2 (`|GetDataTableRow` (`self.Data Table`) (`self.Row Name`))
            (:`then`
              (bind (_dialogue _row _datatable _enddialogue_) (break `/Game/T1/Mechanics/DialogueSystem/Dialogue_Structure` _returnvalue_2))
              (`/Game/T1/Mechanics/DialogueSystem/WB_Dialogue.Update Dialogue` (`self.WidgetDialogue`) _dialogue)
              (set `self.Row Name` _row)
              (set `self.Data Table` _datatable)
              (set `self.EndDialogue` _enddialogue_))))
        (:`Is Not Valid`
          (bind _returnvalue_3 (`|GetDataTableRow` (`self.Data Table`) (`self.Row Name`))
            (:`then`
              (bind (_dialogue_2 _row_2 _datatable_2 _enddialogue__2 _openendeddialogue_ _openendeddialogueoptions) (break `/Game/T1/Mechanics/DialogueSystem/Dialogue_Structure` _returnvalue_3))
              (bind _returnvalue_4 (`|CreateWidget` "/Game/T1/Mechanics/DialogueSystem/WB_Dialogue.WB_Dialogue_C" null (`KismetTextLibrary.Conv_NameToText` (`self.Name`)) _dialogue_2))
              (bind _output_get (set `self.WidgetDialogue` _returnvalue_4))
              (`UserWidget.AddToViewport` _output_get 0)
              (set `self.Row Name` _row_2)
              (set `self.Data Table` _datatable_2)
              (set `self.EndDialogue` _enddialogue__2)
              (`WidgetBlueprintLibrary.SetInputMode_GameAndUIEx` _returnvalue null)
              (set `PlayerController.bShowMouseCursor` true _returnvalue)
              (if _openendeddialogue_
                (for _array_element _openendeddialogueoptions
                  (bind (_optionname _row_3 _datatable_3) (break `/Game/T1/Mechanics/DialogueSystem/OptionsDialogue_Structure` _array_element))
                  (bind _returnvalue_5 (`|CreateWidget` "/Game/T1/Mechanics/DialogueSystem/WB_Options.WB_Options_C" null (`KismetTextLibrary.Conv_NameToText` _optionname) self _row_3 _datatable_3))
                  (`PanelWidget.AddChild` (`/Game/T1/Mechanics/DialogueSystem/WB_Dialogue.OptionScrollBox` (`self.WidgetDialogue`)) _returnvalue_5))))))))))

(event `Option selected`
  (params (RowName :type Name) (DataTable :type "DataTable Object Reference"))
  (bind _widgetdialogue (`self.WidgetDialogue`))
  (bind _returnvalue (`|GetDataTableRow` DataTable RowName)
    (:`then`
      (`PanelWidget.ClearChildren` (`/Game/T1/Mechanics/DialogueSystem/WB_Dialogue.OptionScrollBox` _widgetdialogue))
      (bind (_dialogue _row _datatable _enddialogue_) (break `/Game/T1/Mechanics/DialogueSystem/Dialogue_Structure` _returnvalue))
      (`/Game/T1/Mechanics/DialogueSystem/WB_Dialogue.Update Dialogue` _widgetdialogue _dialogue)
      (set `self.Row Name` _row)
      (set `self.Data Table` _datatable)
      (set `self.EndDialogue` _enddialogue_))))